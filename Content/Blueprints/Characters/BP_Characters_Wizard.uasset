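; BP_Characters_Wizard is the wizard character Blueprint, which manages its own character selection widget.
; SetupUI creates a UI_CharSelect widget, adds it to the viewport, then passes itself in as the widget's Char reference.
; ClearUI removes the stored widget from its parent and clears the reference if it is valid.
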(event `self.SetupUI`
  (bind _returnvalue (`|CreateWidget` "/Game/Blueprints/UI/Selection/UI_CharSelect.UI_CharSelect_C"))
  (bind _output_get (set `self.CharSelect` _returnvalue))
  (`UserWidget.AddToViewport` _output_get 0)
  (set `/Game/Blueprints/UI/Selection/UI_CharSelect.Char` self (`self.CharSelect`)))

(event `self.ClearUI`
  (bind _charselect (`self.CharSelect`))
  (`/Engine/EditorBlueprintResources/StandardMacros.IsValid` _charselect
    (:`Is Valid`
      (`Widget.RemoveFromParent` _charselect)
      (set `self.CharSelect` null))))

(fn `UserConstructionScript`)