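; BP_PlayerController is the player controller that swaps on-screen UI between a tile phase and a game phase.
; On BeginPlay it sets game-and-UI input with the mouse locked in fullscreen and visible during capture.
; TilePhaseUI shows the tile phase and begin-level widgets, while GamePhaseUI shows the game phase widget, each removing the other phase's widgets.
; An unconnected debug trace for printing the actor under the cursor never runs.
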(event `Key|LeftMouseButton`
  (params (Key :type "Key Structure")))

(event `self.ReceiveBeginPlay`
  (`WidgetBlueprintLibrary.SetInputMode_GameAndUIEx` self null "LockInFullscreen" false))

(event `self.TilePhaseUI`
  (bind _gamephaseuibp (`self.GamePhaseUIBP`))
  (bind _returnvalue (`|CreateWidget` "/Game/Blueprints/UI/TilePhase/UI_TilePhase.UI_TilePhase_C"))
  (bind _output_get (set `self.TilePhaseUIBP` _returnvalue))
  (`UserWidget.AddToViewport` _output_get 0)
  (bind _returnvalue_2 (`|CreateWidget` "/Game/Blueprints/UI/TilePhase/UI_BeginLevel.UI_BeginLevel_C"))
  (bind _output_get_2 (set `self.PlayButtonUI` _returnvalue_2))
  (`UserWidget.AddToViewport` _output_get_2 0)
  (`/Engine/EditorBlueprintResources/StandardMacros.IsValid` _gamephaseuibp
    (:`Is Valid`
      (`Widget.RemoveFromParent` _gamephaseuibp)
      (set `self.GamePhaseUIBP` null))))

(event `self.GamePhaseUI`
  (bind _tilephaseuibp (`self.TilePhaseUIBP`))
  (bind _playbuttonui (`self.PlayButtonUI`))
  (bind _returnvalue (`|CreateWidget` "/Game/Blueprints/UI/GamePhase/UI_GamePhase.UI_GamePhase_C"))
  (bind _output_get (set `self.GamePhaseUIBP` _returnvalue))
  (`UserWidget.AddToViewport` _output_get 0)
  (`/Engine/EditorBlueprintResources/StandardMacros.IsValid` _tilephaseuibp
    (:`Is Valid`
      (`Widget.RemoveFromParent` _tilephaseuibp)
      (set `self.TilePhaseUIBP` null))
    (:`Is Not Valid`
      _))
  (`/Engine/EditorBlueprintResources/StandardMacros.IsValid` _playbuttonui
    (:`Is Valid`
      (`Widget.RemoveFromParent` _playbuttonui)
      (set `self.PlayButtonUI` null))))

(fn `UserConstructionScript`)