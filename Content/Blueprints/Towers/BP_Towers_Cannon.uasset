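; BP_Towers_Cannon is a cannon tower Blueprint that manages its own selection UI.
; SetupUI creates a UI_TowerSelect widget, adds it to the viewport, then passes the tower itself to the widget's Tower variable.
; ClearUI removes the stored widget from its parent and clears the reference if it is valid.
; The file holds no firing or targeting logic, and its construction script is empty.
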(event `self.SetupUI`
  (bind _returnvalue (`|CreateWidget` "/Game/Blueprints/UI/Selection/UI_TowerSelect.UI_TowerSelect_C"))
  (bind _output_get (set `self.TowerSelect` _returnvalue))
  (`UserWidget.AddToViewport` _output_get 0)
  (set `/Game/Blueprints/UI/Selection/UI_TowerSelect.Tower` self (`self.TowerSelect`)))

(event `self.ClearUI`
  (bind _towerselect (`self.TowerSelect`))
  (`/Engine/EditorBlueprintResources/StandardMacros.IsValid` _towerselect
    (:`Is Valid`
      (`Widget.RemoveFromParent` _towerselect)
      (set `self.TowerSelect` null))))

(fn `UserConstructionScript`)